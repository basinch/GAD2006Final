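; Player controller that handles the pause menu for the player's BP_NetAvatar, which it caches on BeginPlay.
; The J key replaces all widgets with W_PauseMenu, shows the cursor and freezes play through zero global time dilation.
; Edits to the menu's character-creation text box update the avatar's TextRender live.
; Unpausing delegates to BP_BaseGameMode's StartGame, leaving an older inline camera, input and HUD restore chain disconnected.
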(event `self.ReceiveBeginPlay`
  (bind _asbp_net_avatar (cast `/Game/Blueprints/BP_NetAvatar` (`GameplayStatics.GetPlayerCharacter` 0)))
  (set `self.As BP Net Avatar` _asbp_net_avatar))

(event `Key|J`
  (params (Key :type "Key Structure"))
  ;[1 1 1] Pause Logic
  (:`Pressed`
    (`/Engine/EditorBlueprintResources/StandardMacros.IsValid` (`self.PauseMenuWidget`)
      (:`Is Valid`
        (`self.Resume`))
      (:`Is Not Valid`
        (`WidgetLayoutLibrary.RemoveAllWidgets`)
        (bind _returnvalue (`|CreateWidget` "/Game/Blueprints/UMG/W_PauseMenu.W_PauseMenu_C"))
        (bind _output_get (set `self.PauseMenuWidget` _returnvalue))
        (add `EditableText.OnTextChanged` (`/Game/Blueprints/UMG/W_CharCreation.EditableText_0` (`/Game/Blueprints/UMG/W_CharCustomization.W_CharCreation` (`/Game/Blueprints/UMG/W_PauseMenu.W_CharCustomization` _output_get))) (delegate `OnTextChanged_Event`))
        (set `self.bShowMouseCursor` true)
        (`WidgetBlueprintLibrary.SetInputMode_GameAndUIEx` self _output_get "DoNotLock" false)
        (`UserWidget.AddToViewport` (`self.PauseMenuWidget`) 0)
        (`GameplayStatics.SetGlobalTimeDilation` 0.0)))))

(event `OnTextChanged_Event`
  (params (Text :type "Text (by ref)"))
  ;[1 1 1] Pause Logic
  (`TextRenderComponent.K2_SetText` (`/Game/Blueprints/BP_NetAvatar.TextRender` (`self.As BP Net Avatar`)) Text))

(event `/Game/BI_Pause.UnPause`
  ;[1 1 1] Pause Logic
  (`self.Resume`))

(event `Resume`
  ;[1 1 1] Pause Logic
  (`/Game/BP_BaseGameMode.StartGame` (cast `/Game/BP_BaseGameMode` (`GameplayStatics.GetGameMode`) :!pure true)))

(fn `UserConstructionScript`)